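; Enemy formation spawner that builds a grid of BP_Enemy actors and marches it as one block in a Space Invaders style.
; On BeginPlay, Childs spawns the horizontally offset grid, colors each row by material, attaches every enemy and gives it a spawner reference.
; Tick slides the root along Y per CurrentMovement; a Down state, not set here, drops it one step and switches to NextMovement, alternating left and right.
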(event `self.ReceiveBeginPlay`
  (`self.Childs`))

(event `self.ReceiveTick`
  (params (DeltaSeconds :type "Float (single-precision)"))
  (set `self.DeltaSeconds` DeltaSeconds)
  (switch `/Game/Blueprint/Enemy/ENUM_MovementEnemy` (`self.CurrentMovement`)
    (:`NewEnumerator0`
      (set `self.MovementMultiplayer` 1.0)
      (`SceneComponent.K2_AddRelativeLocation` (`self.DefaultSceneRoot`) (`KismetMathLibrary.MakeVector` 0.0 (* (`self.DeltaSeconds`) (`self.MovementSpeed`) (`self.MovementMultiplayer`))) false false :!label _label))
    (:`NewEnumerator1`
      (set `self.MovementMultiplayer` -1.0)
      (goto _label))
    (:`NewEnumerator2`
      (set `self.CurrentMovement` (`self.NextMovement`))
      (switch `/Game/Blueprint/Enemy/ENUM_MovementEnemy` (`self.CurrentMovement`)
        (:`NewEnumerator0`
          (set `self.NextMovement` "NewEnumerator1"))
        (:`NewEnumerator1`
          (set `self.NextMovement` "NewEnumerator0")))
      (`SceneComponent.K2_AddRelativeLocation` (`self.DefaultSceneRoot`) (0.0 0.0 -50.0) false false))))

(fn `Childs`
  (locals (CurrentCollumn :type Integer) (CurrentRow :type Integer) (DistanceBetweenEnemy :type Integer :default 150) (EnemySize :type Integer :default 100))
  (for _index (range (+ (`self.MaxRow`) 1))
    (set `local.CurrentRow` _index)
    (for _index_2 (range (+ (`self.MaxCollumn`) 1))
      (set `local.CurrentCollumn` _index_2)
      (bind _returnvalue (`|SpawnActorFromClass` "/Game/Blueprint/Enemy/BP_Enemy.BP_Enemy_C" (`KismetMathLibrary.MakeTransform` (`KismetMathLibrary.MakeVector` 0.0 (- (`KismetMathLibrary.Conv_IntToDouble` (* (`local.CurrentCollumn`) (`local.DistanceBetweenEnemy`))) (* (`KismetMathLibrary.Conv_IntToDouble` (+ (* (`local.DistanceBetweenEnemy`) (`self.MaxCollumn`)) (`local.EnemySize`))) 0.5)) (`KismetMathLibrary.Conv_IntToDouble` (* (`local.CurrentRow`) (`local.DistanceBetweenEnemy`)))) (struct) (1.0 1.0 1.0)) "Undefined" "OverrideRootScale" null null))
      (`self.SetEnemyMaterial` (`local.CurrentRow`) _returnvalue)
      (set `/Game/Blueprint/Enemy/BP_Enemy.EnemySpawner` self _returnvalue)
      (`self.K2_AttachToActor` _returnvalue self "None" "KeepRelative" "KeepRelative" "KeepRelative" true))))

(fn `SetEnemyMaterial`
  (params (InRow :type Integer) (InEnemyObject :type "/Game/Blueprint/Enemy/BP_Enemy Object Reference"))
  (`PrimitiveComponent.SetMaterial` (`/Game/Blueprint/Enemy/BP_Enemy.Cube` InEnemyObject) 0 (select `int` (`local.InRow`) :`0` "/Game/Art/MI_Color_Blue.MI_Color_Blue" :`1` "/Game/Art/MI_Color_Green.MI_Color_Green" :`2` "/Game/Art/MI_Color_Purple.MI_Color_Purple" :`3` "/Game/Art/MI_Color_Red.MI_Color_Red" :`4` "/Game/Art/MI_Color_Yellow.MI_Color_Yellow" :!type "MaterialInterface Object Reference"))
  (return))

(fn `UserConstructionScript`)